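; BP_Spaceship is the spaceship actor that the player assembles piece by piece from five static mesh parts.
; Box overlaps track whether the first-person character is in range and hand it a reference to the ship.
; The add_element event passes a piece number through AddElem, which reveals the matching mesh, enables its blocking collision, plays particle and sound effects, and updates that slot in the character's SpaceOwne array.
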(event OnComponentBeginOverlap(Box)
  (params (OverlappedComponent :type Primitive%20Component%20Object%20Reference) (OtherActor :type Actor%20Object%20Reference) (OtherComp :type Primitive%20Component%20Object%20Reference) (OtherBodyIndex :type Integer) (bFromSweep :type Boolean) (SweepResult :type Hit%20Result%20Structure%20%28by%20ref%29))
  (bind _asbp_first_person_character (Utilities|Casting|CastToBP_FirstPersonCharacter OtherActor))
  (Variables|Default|SetIn_box_SpaceShip true)
  (Variables|/Game/LostRocket/Character/BP_FirstPersonCharacter.BP_FirstPersonCharacter_C|SetBP_Spaceship _asbp_first_person_character self)
  (Variables|Default|Setbp_FirstPerson _asbp_first_person_character))

(event OnComponentEndOverlap(Box)
  (params (OverlappedComponent :type Primitive%20Component%20Object%20Reference) (OtherActor :type Actor%20Object%20Reference) (OtherComp :type Primitive%20Component%20Object%20Reference) (OtherBodyIndex :type Integer))
  (bind _asbp_first_person_character (Utilities|Casting|CastToBP_FirstPersonCharacter OtherActor))
  (Variables|Default|SetIn_box_SpaceShip false)
  (Variables|/Game/LostRocket/Character/BP_FirstPersonCharacter.BP_FirstPersonCharacter_C|SetBP_Spaceship _asbp_first_person_character self))

(event Custom|add_element
  (params (NewParam :type Integer))
  (CallFunction|AddElem (Variables|Default|GetStaticMesh1) NewParam)
  (CallFunction|AddElem (Variables|Default|GetStaticMesh2) NewParam 1)
  (CallFunction|AddElem (Variables|Default|GetStaticMesh3) NewParam 2)
  (CallFunction|AddElem (Variables|Default|GetStaticMesh4) NewParam 3)
  (CallFunction|AddElem (Variables|Default|GetStaticMesh5) NewParam 4))

(event EventBeginPlay)

(event Collision|EventActorBeginOverlap
  (params (OtherActor :type Actor%20Object%20Reference)))

(event EventTick
  (params (DeltaSeconds :type Float%20%28single-precision%29)))

(fn ConstructionScript)

(fn AddElem
  (params (Mesh :type Scene%20Component%20Object%20Reference) (Piece_Number :type Integer) (Index :type Integer))
  (bind _asstatic_mesh_component (Utilities|Casting|CastToStaticMeshComponent Mesh))
  (if (== Piece_Number Index)
    (Rendering|SetVisibility _asstatic_mesh_component true false)
    (Collision|SetCollisionProfileName _asstatic_mesh_component "BlockAllDynamic" true :!class /Script/Engine.PrimitiveComponent)
    (Components|Activation|Activate (Variables|Default|GetP_FrostGiant_Trap_Target) false)
    (Audio|PlaySound2D "/Game/LostRocket/DynamicObject/Spaceship_part/spaceship_tp.spaceship_tp" 1.0 0.6 0.0 0 0)
    (Utilities|Array|SetArrayElem (Variables|/Game/LostRocket/Character/BP_FirstPersonCharacter.BP_FirstPersonCharacter_C|GetSpace_Owne (Variables|Default|Getbp_FirstPerson)) Piece_Number false)))