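; BP_spaceship_piece1 is a collectible spaceship part that the first-person character can pick up.
; Its Box overlap flags the character as in range, hands it a reference to the piece, and toggles custom depth on the mesh, likely for highlighting.
; The Pick_up event, not triggered within this graph, activates an effect, plays a pitched-down teleport sound, then destroys the actor after a delay.
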(event OnComponentBeginOverlap(Box)
  (params (OverlappedComponent :type Primitive%20Component%20Object%20Reference) (OtherActor :type Actor%20Object%20Reference) (OtherComp :type Primitive%20Component%20Object%20Reference) (OtherBodyIndex :type Integer) (bFromSweep :type Boolean) (SweepResult :type Hit%20Result%20Structure%20%28by%20ref%29))
  (bind _asbp_first_person_character (Utilities|Casting|CastToBP_FirstPersonCharacter OtherActor))
  (Variables|/Game/LostRocket/Character/BP_FirstPersonCharacter.BP_FirstPersonCharacter_C|SetIn_SpaceshipPiece _asbp_first_person_character true)
  (Variables|/Game/LostRocket/Character/BP_FirstPersonCharacter.BP_FirstPersonCharacter_C|SetBP_Spaceship_Piece _asbp_first_person_character self)
  (Rendering|SetRenderCustomDepth (Variables|Default|GetStaticMesh) true))

(event OnComponentEndOverlap(Box)
  (params (OverlappedComponent :type Primitive%20Component%20Object%20Reference) (OtherActor :type Actor%20Object%20Reference) (OtherComp :type Primitive%20Component%20Object%20Reference) (OtherBodyIndex :type Integer))
  (bind _asbp_first_person_character (Utilities|Casting|CastToBP_FirstPersonCharacter OtherActor))
  (Variables|/Game/LostRocket/Character/BP_FirstPersonCharacter.BP_FirstPersonCharacter_C|SetIn_SpaceshipPiece _asbp_first_person_character false)
  (Rendering|SetRenderCustomDepth (Variables|Default|GetStaticMesh) false))

(event Custom|Pick_up
  (Components|Activation|Activate (Variables|Default|GetP_FrostGiant_Trap_Target) false)
  (Audio|PlaySound2D "/Game/LostRocket/DynamicObject/Spaceship_part/spaceship_tp.spaceship_tp" 1.0 0.6 0.0 0 0)
  (Utilities|FlowControl|Delay 4.0)
  (Actor|DestroyActor))

(event EventBeginPlay)

(event Collision|EventActorBeginOverlap
  (params (OtherActor :type Actor%20Object%20Reference)))

(event EventTick
  (params (DeltaSeconds :type Float%20%28single-precision%29)))

(fn ConstructionScript)