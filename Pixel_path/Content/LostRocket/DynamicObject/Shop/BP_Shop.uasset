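; BP_Shop is a shop terminal actor that links the first-person player to a WB_Shop interface.
; Its trigger box registers the shop on the character, shows the shop and interaction widgets, and outlines the terminal via custom depth.
; The widget component's WB_Shop instance gets a back-reference and can be moved on and off the viewport.
; Set_camera exits shop mode, restoring HUD, walking, saved camera transform and game-only input.
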(event OnComponentBeginOverlap(Box)
  (params (OverlappedComponent :type Primitive%20Component%20Object%20Reference) (OtherActor :type Actor%20Object%20Reference) (OtherComp :type Primitive%20Component%20Object%20Reference) (OtherBodyIndex :type Integer) (bFromSweep :type Boolean) (SweepResult :type Hit%20Result%20Structure%20%28by%20ref%29))
  (bind _asbp_first_person_character (Utilities|Casting|CastToBP_FirstPersonCharacter OtherActor))
  (Variables|Default|SetIn_box true)
  (Variables|/Game/LostRocket/Character/BP_FirstPersonCharacter.BP_FirstPersonCharacter_C|SetBP_Shop _asbp_first_person_character self)
  (Rendering|SetVisibility (Variables|Default|GetWidget) true false)
  (Rendering|SetVisibility (Variables|Default|GetWidget_Interraction) true false)
  (Rendering|SetRenderCustomDepth (Variables|Default|GetSM_Terminal_1) true))

(event OnComponentEndOverlap(Box)
  (params (OverlappedComponent :type Primitive%20Component%20Object%20Reference) (OtherActor :type Actor%20Object%20Reference) (OtherComp :type Primitive%20Component%20Object%20Reference) (OtherBodyIndex :type Integer))
  (bind _asbp_first_person_character (Utilities|Casting|CastToBP_FirstPersonCharacter OtherActor))
  (Variables|Default|SetIn_box false)
  (Variables|/Game/LostRocket/Character/BP_FirstPersonCharacter.BP_FirstPersonCharacter_C|SetBP_Shop _asbp_first_person_character 0)
  (Rendering|SetVisibility (Variables|Default|GetWidget) false false)
  (Rendering|SetVisibility (Variables|Default|GetWidget_Interraction) false false)
  (Rendering|SetRenderCustomDepth (Variables|Default|GetSM_Terminal_1) false))

(event Custom|Set_camera
  (bind _returnvalue (Game|GetPlayerController 0))
  (bind _bp_firstperson (Variables|Default|GetBP_FirstPerson))
  (bind _firstpersoncamera (Variables|/Game/LostRocket/Character/BP_FirstPersonCharacter.BP_FirstPersonCharacter_C|GetFirstPersonCamera _bp_firstperson))
  (Variables|/Game/LostRocket/Character/BP_FirstPersonCharacter.BP_FirstPersonCharacter_C|SetIn_Widget _bp_firstperson false)
  (Widget|SetVisibility (Variables|/Game/LostRocket/Character/BP_FirstPersonCharacter.BP_FirstPersonCharacter_C|GetWB_Player_Hud _bp_firstperson) "Visible")
  (Variables|/Game/LostRocket/Character/BP_FirstPersonCharacter.BP_FirstPersonCharacter_C|SetWB_Shop _bp_firstperson 0)
  (Pawn|Components|CharacterMovement|SetMovementMode (Variables|/Script/Engine.Character|GetCharacterMovement _bp_firstperson) "MOVE_Walking" 0)
  (Variables|/Script/Engine.CameraComponent|SetbUsePawnControlRotation _firstpersoncamera true)
  (Transformation|SetRelativeTransform _firstpersoncamera (Variables|/Game/LostRocket/Character/BP_FirstPersonCharacter.BP_FirstPersonCharacter_C|GetLast_pos _bp_firstperson) false false)
  (Variables|/Script/Engine.PlayerController|SetbShowMouseCursor _returnvalue false)
  (Input|SetInputModeGameOnly _returnvalue false)
  (Rendering|SetVisibility (Variables|Default|GetWidget) true false))

(event Custom|Remove_from_viewport
  (Widget|RemovefromParent (Variables|Default|GetWB_Shop)))

(event Custom|Add_to_viewport
  (UserInterface|Viewport|AddtoViewport (Variables|Default|GetWB_Shop) 0))

(event EventBeginPlay
  (bind _asbp_first_person_character (Utilities|Casting|CastToBP_FirstPersonCharacter (Game|GetPlayerCharacter 0)))
  (Variables|Default|SetBP_FirstPerson _asbp_first_person_character)
  (bind _aswb_shop (Utilities|Casting|CastToWB_Shop (UserInterface|GetUserWidgetObject (Variables|Default|GetWidget))))
  (Variables|Default|SetWB_Shop _aswb_shop)
  (Variables|/Game/LostRocket/DynamicObject/Shop/WB_Shop.WB_Shop_C|SetBP_shop _aswb_shop self))

(fn ConstructionScript)