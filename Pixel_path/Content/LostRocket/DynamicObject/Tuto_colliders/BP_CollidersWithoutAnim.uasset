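; BP_CollidersWithoutAnim is a trigger volume that shows a timed tutorial to the first-person character.
; On the first box overlap by that character, it sets the character's InWidget flag and adds a WBP_Tutorial widget to the viewport, loaded with its Index and Duration.
; After Duration elapses it removes the widget and clears the flag; a DoOnce keeps it from repeating.
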(event OnComponentBeginOverlap(Box)
  (params (OverlappedComponent :type Primitive%20Component%20Object%20Reference) (OtherActor :type Actor%20Object%20Reference) (OtherComp :type Primitive%20Component%20Object%20Reference) (OtherBodyIndex :type Integer) (bFromSweep :type Boolean) (SweepResult :type Hit%20Result%20Structure%20%28by%20ref%29))
  (bind _duration (Variables|Default|GetDuration))
  (bind _asbp_first_person_character (Utilities|Casting|CastToBP_FirstPersonCharacter OtherActor))
  (Utilities|FlowControl|DoOnce false
    (:Completed
      (bind _output_get (Variables|Default|SetBP_firstPerson _asbp_first_person_character))
      (Variables|/Game/LostRocket/Character/BP_FirstPersonCharacter.BP_FirstPersonCharacter_C|SetIn_Widget _output_get true)
      (bind _returnvalue (UserInterface|CreateWidget "/Game/LostRocket/Character/HUD/TutorialPopup/WBP_Tutorial.WBP_Tutorial_C"))
      (UserInterface|Viewport|AddtoViewport _returnvalue 0)
      (Default|LoadTutorial _returnvalue _duration (Variables|Default|GetIndex))
      (Utilities|FlowControl|Delay _duration)
      (Widget|RemovefromParent _returnvalue)
      (Variables|/Game/LostRocket/Character/BP_FirstPersonCharacter.BP_FirstPersonCharacter_C|SetIn_Widget (Variables|Default|GetBP_firstPerson) false))))

(event EventBeginPlay)

(event Collision|EventActorBeginOverlap
  (params (OtherActor :type Actor%20Object%20Reference)))

(event EventTick
  (params (DeltaSeconds :type Float%20%28single-precision%29)))

(fn ConstructionScript)