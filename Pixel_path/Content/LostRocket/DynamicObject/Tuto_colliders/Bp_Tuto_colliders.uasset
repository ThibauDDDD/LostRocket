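; Tutorial trigger volume that plays a one-time cinematic tutorial when the first-person character enters its box.
; On overlap it hides the player HUD, disables movement, switches to UI-only input, plays its level sequence and loads a WBP_Tutorial widget by Index.
; A Delay of Duration, rather than the sequence finishing, times the return to walking and game input, the EndOfCinematics call and the widget's removal.
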(event OnComponentBeginOverlap(Box)
  (params (OverlappedComponent :type Primitive%20Component%20Object%20Reference) (OtherActor :type Actor%20Object%20Reference) (OtherComp :type Primitive%20Component%20Object%20Reference) (OtherBodyIndex :type Integer) (bFromSweep :type Boolean) (SweepResult :type Hit%20Result%20Structure%20%28by%20ref%29))
  (bind _duration (Variables|Default|GetDuration))
  (bind _asbp_first_person_character (Utilities|Casting|CastToBP_FirstPersonCharacter OtherActor))
  (Utilities|FlowControl|DoOnce false
    (:Completed
      (bind _output_get (Variables|Default|SetBP_firstPerson _asbp_first_person_character))
      (Variables|/Game/LostRocket/Character/BP_FirstPersonCharacter.BP_FirstPersonCharacter_C|SetIn_Widget _output_get true)
      (Variables|/Script/UMG.Widget|SetVisibility (Variables|/Game/LostRocket/Character/BP_FirstPersonCharacter.BP_FirstPersonCharacter_C|GetWB_Player_Hud _asbp_first_person_character) "Hidden")
      (bind _returnvalue (UserInterface|CreateWidget "/Game/LostRocket/Character/HUD/TutorialPopup/WBP_Tutorial.WBP_Tutorial_C"))
      (UserInterface|Viewport|AddtoViewport _returnvalue 0)
      (Pawn|Components|CharacterMovement|DisableMovement (Variables|/Script/Engine.Character|GetCharacterMovement _asbp_first_person_character))
      (Input|SetInputModeUIOnly (Game|GetPlayerController 0) 0 "DoNotLock" false)
      (bind _returnvalue_2 (Sequencer|Player|CreateLevelSequencePlayer (Variables|Default|GetLevel%20Sequence)))
      (Sequencer|Player|Play _returnvalue_2 :!class /Script/MovieScene.MovieSceneSequencePlayer)
      (Default|LoadTutorial _returnvalue _duration (Variables|Default|GetIndex))
      (Utilities|FlowControl|Delay _duration)
      (Pawn|Components|CharacterMovement|SetMovementMode (Variables|/Script/Engine.Character|GetCharacterMovement (Variables|Default|GetBP_firstPerson)) "MOVE_Walking" 0)
      (Input|SetInputModeGameOnly (Game|GetPlayerController 0) false)
      (Default|EndOfCinematics (Variables|Default|GetBP_firstPerson))
      (Widget|RemovefromParent _returnvalue)
      (Variables|/Game/LostRocket/Character/BP_FirstPersonCharacter.BP_FirstPersonCharacter_C|SetIn_Widget (Variables|Default|GetBP_firstPerson) false))))

(event EventBeginPlay)

(event Collision|EventActorBeginOverlap
  (params (OtherActor :type Actor%20Object%20Reference)))

(event EventTick
  (params (DeltaSeconds :type Float%20%28single-precision%29)))

(fn ConstructionScript)