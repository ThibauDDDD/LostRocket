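; BP_DamageObject is a one-shot hazard actor that damages the first-person player character on contact.
; Any hit on its cube mesh destroys the actor, whatever it strikes.
; If the other actor is BP_FirstPersonCharacter, it subtracts Damage directly from that character's Health.
; It then prints the remaining Health, or "Dead" at zero or below, with no further death handling here.
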(event OnComponentHit(SM_ChamferCube)
  (params (HitComponent :type Primitive%20Component%20Object%20Reference) (OtherActor :type Actor%20Object%20Reference) (OtherComp :type Primitive%20Component%20Object%20Reference) (NormalImpulse :type Vector :default "0, 0, 0") (Hit :type Hit%20Result%20Structure%20%28by%20ref%29))
  (Actor|DestroyActor)
  (bind _asbp_first_person_character (Utilities|Casting|CastToBP_FirstPersonCharacter OtherActor))
  (bind _output_get (Variables|/Game/LostRocket/Character/BP_FirstPersonCharacter.BP_FirstPersonCharacter_C|SetHealth _asbp_first_person_character (- (Variables|/Game/LostRocket/Character/BP_FirstPersonCharacter.BP_FirstPersonCharacter_C|GetHealth _asbp_first_person_character) (Variables|Default|GetDamage))))
  (if (<= _output_get 0)
    (Development|PrintString "Dead")
    (else
      (Development|PrintString (Utilities|String|ToString(Integer) _output_get)))))

(fn ConstructionScript)