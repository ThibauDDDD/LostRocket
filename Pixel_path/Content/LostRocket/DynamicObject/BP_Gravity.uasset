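; BP_Gravity is a single-use cube that permanently shifts the first-person character's gravity scale on contact.
; When BP_FirstPersonCharacter hits the cube mesh, the GravityType flag selects whether the Gravity amount is added to or subtracted from the movement component's current GravityScale.
; Two small helper functions do the math, and the actor destroys itself afterward.
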(event OnComponentHit(SM_ChamferCube)
  (params (HitComponent :type Primitive%20Component%20Object%20Reference) (OtherActor :type Actor%20Object%20Reference) (OtherComp :type Primitive%20Component%20Object%20Reference) (NormalImpulse :type Vector :default "0, 0, 0") (Hit :type Hit%20Result%20Structure%20%28by%20ref%29))
  (bind _gravity (Variables|Default|GetGravity))
  (bind _asbp_first_person_character (Utilities|Casting|CastToBP_FirstPersonCharacter OtherActor))
  (Variables|Default|SetCharacterGravityScale (Variables|/Script/Engine.CharacterMovementComponent|GetGravityScale (Variables|/Script/Engine.Character|GetCharacterMovement _asbp_first_person_character)))
  (if (Variables|Default|GetGravityType)
    (bind __ (Utilities|AddGravityScale (Variables|Default|GetCharacterGravityScale) _gravity)
      (:%20%20%20
        (Variables|/Script/Engine.CharacterMovementComponent|SetGravityScale (Variables|/Script/Engine.Character|GetCharacterMovement _asbp_first_person_character) __)))
    (else
      (bind ______ (Utilities|SubGravityScale (Variables|Default|GetCharacterGravityScale) _gravity)
        (:%20%20%20
          (Variables|/Script/Engine.CharacterMovementComponent|SetGravityScale (Variables|/Script/Engine.Character|GetCharacterMovement _asbp_first_person_character) ______)))))
  (Actor|DestroyActor))

(fn ConstructionScript)