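; Seamless linked portal actor that shows the view through its partner and teleports the first-person player, optionally ending the level.
; Setup, rerun whenever the portal moves, feeds the linked portal's clip-planed scene capture into a dynamic material through a viewport-sized render target.
; Each tick mirrors the player camera onto the linked capture and checks for front-to-back plane crossings.
; Crossing plays audio and transfers position, rotation and velocity into the partner's space.
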(event Custom|CustomEvent
  (bind _returnvalue (Viewport|GetViewportSize))
  (bind _forwarddirection (Variables|Default|GetForwardDirection))
  (bind _offsetamount (Variables|Default|GetOffsetAmount))
  (bind _returnvalue_2 (Math|Vector|GetForwardVector _forwarddirection))
  (bind _returnvalue_3 (* _returnvalue_2 _offsetamount))
  (bind (_x _y _z) (Math|Vector|BreakVector _returnvalue_3))
  (Variables|Default|SetPos (Transformation|GetActorLocation))
  (bind _returnvalue_4 (Rendering|Material|CreateDynamicMaterialInstance "/Game/LostRocket/DynamicObject/Portal/M_Portal.M_Portal" "None" "None" :!class /Script/Engine.KismetMaterialLibrary))
  (bind _output_get (Variables|Default|SetPortal_Mat _returnvalue_4))
  (Rendering|Material|SetMaterial (Variables|Default|GetPortalPlane) 0 _output_get)
  (bind _returnvalue_5 (Rendering|CreateRenderTarget2D (Math|Float|Truncate (.x _returnvalue)) (Math|Float|Truncate (.y _returnvalue)) "RTF_RGBA16f"))
  (bind _output_get_2 (Variables|Default|SetPortal_RT _returnvalue_5))
  (Rendering|Material|SetTextureParameterValue (Variables|Default|GetPortal_Mat) "Texture" _output_get_2)
  (Variables|/Script/Engine.SceneCaptureComponent2D|SetTextureTarget (Variables|BP_Portal1_C|GetPortalCamera (Variables|Default|GetLinked%20portal)) (Variables|Default|GetPortal_RT))
  (CallFunction|SetClipPlanes)
  (Rendering|Material|SetVectorParameterValue (Variables|Default|GetPortal_Mat) "OffsetDistance" (Math|Color|MakeColor _x _y _z) :!class /Script/Engine.MaterialInstanceDynamic))

(event EventBeginPlay
  (bind _returnvalue (Viewport|GetViewportSize))
  (bind _forwarddirection (Variables|Default|GetForwardDirection))
  (bind _offsetamount (Variables|Default|GetOffsetAmount))
  (bind _returnvalue_2 (Math|Vector|GetForwardVector _forwarddirection))
  (bind _returnvalue_3 (* _returnvalue_2 _offsetamount))
  (bind (_x _y _z) (Math|Vector|BreakVector _returnvalue_3))
  (Components|Tick|SetTickGroup "TG_PrePhysics")
  (Variables|Default|SetPos (Transformation|GetActorLocation))
  (bind _returnvalue_4 (Rendering|Material|CreateDynamicMaterialInstance "/Game/LostRocket/DynamicObject/Portal/M_Portal.M_Portal" "None" "None" :!class /Script/Engine.KismetMaterialLibrary))
  (bind _output_get (Variables|Default|SetPortal_Mat _returnvalue_4))
  (Rendering|Material|SetMaterial (Variables|Default|GetPortalPlane) 0 _output_get)
  (bind _returnvalue_5 (Rendering|CreateRenderTarget2D (Math|Float|Truncate (.x _returnvalue)) (Math|Float|Truncate (.y _returnvalue)) "RTF_RGBA16f"))
  (bind _output_get_2 (Variables|Default|SetPortal_RT _returnvalue_5))
  (Rendering|Material|SetTextureParameterValue (Variables|Default|GetPortal_Mat) "Texture" _output_get_2)
  (Variables|/Script/Engine.SceneCaptureComponent2D|SetTextureTarget (Variables|BP_Portal1_C|GetPortalCamera (Variables|Default|GetLinked%20portal)) (Variables|Default|GetPortal_RT))
  (CallFunction|SetClipPlanes)
  (Rendering|Material|SetVectorParameterValue (Variables|Default|GetPortal_Mat) "OffsetDistance" (Math|Color|MakeColor _x _y _z) :!class /Script/Engine.MaterialInstanceDynamic))

(event Collision|EventActorBeginOverlap
  (params (OtherActor :type Actor%20Object%20Reference)))

(event EventTick
  (params (DeltaSeconds :type Float%20%28single-precision%29))
  (if (Class|KismetMathLibrary|EqualExactlyVectorVector (Transformation|GetActorLocation) (Variables|Default|GetPos))
    _
    (else
      (CallFunction|CustomEvent)))
  (CallFunction|UpgradeSceneCapture)
  (CallFunction|Checkviewportsize)
  (CallFunction|ShouldTeleport?))

(fn ConstructionScript)

(fn UpgradeSceneCapture
  (bind _returnvalue (Game|GetPlayerCameraManager 0))
  (bind _returnvalue_2 (Transformation|GetActorTransform))
  (bind _returnvalue_3 (Transformation|GetActorTransform))
  (bind _linked_portal (Variables|Default|GetLinked%20portal))
  (bind _returnvalue_4 (Transformation|GetActorTransform _linked_portal))
  (bind (_location _rotation _scale) (Math|Transform|BreakTransform _returnvalue_3))
  (bind _transformcomponent (Variables|/Script/Engine.PlayerCameraManager|GetTransformComponent _returnvalue))
  (bind _returnvalue_5 (Transformation|GetWorldRotation _transformcomponent))
  (bind (_x _y _z) (Math|Vector|BreakVector _scale))
  (bind (_x_2 _y_2 _z_2) (Math|Rotator|BreakRotIntoAxes _returnvalue_5))
  (Transformation|SetWorldLocationAndRotation (Variables|BP_Portal1_C|GetPortalCamera (Variables|Default|GetLinked%20portal)) (Math|Transform|TransformLocation (Transformation|GetActorTransform (Variables|Default|GetLinked%20portal)) (Math|Transform|InverseTransformLocation (Math|Transform|MakeTransform _location _rotation (Math|Vector|MakeVector (* _x -1.0) (* _y -1.0) _z)) (Transformation|GetWorldLocation (Variables|/Script/Engine.PlayerCameraManager|GetTransformComponent (Game|GetPlayerCameraManager 0))))) (Math|Rotator|MakeRotationfromAxes (Math|Transform|TransformDirection _returnvalue_4 (Math|Vector|MirrorVectorbyNormal (Math|Vector|MirrorVectorbyNormal (Math|Transform|InverseTransformDirection _returnvalue_2 _x_2) "1.000000,0.000000,0.000000") "0.000000,1.000000,0.000000")) (Math|Transform|TransformDirection _returnvalue_4 (Math|Vector|MirrorVectorbyNormal (Math|Vector|MirrorVectorbyNormal (Math|Transform|InverseTransformDirection _returnvalue_2 _y_2) "1.000000,0.000000,0.000000") "0.000000,1.000000,0.000000")) (Math|Transform|TransformDirection _returnvalue_4 (Math|Vector|MirrorVectorbyNormal (Math|Vector|MirrorVectorbyNormal (Math|Transform|InverseTransformDirection _returnvalue_2 _z_2) "1.000000,0.000000,0.000000") "0.000000,1.000000,0.000000"))) false false))

(fn SetClipPlanes
  (bind _portalcamera (Variables|Default|GetPortalCamera))
  (Utilities|IsValid (Variables|Default|GetLinked%20portal)
    (:Is%20Valid
      (Variables|/Script/Engine.SceneCaptureComponent2D|SetbEnableClipPlane _portalcamera true)
      (Variables|/Script/Engine.SceneCaptureComponent2D|SetClipPlaneBase _portalcamera (+ (Transformation|GetWorldLocation (Variables|Default|GetPortalPlane)) (* (Math|Vector|GetForwardVector (Variables|Default|GetForwardDirection)) -3.0)))
      (Variables|/Script/Engine.SceneCaptureComponent2D|SetClipPlaneNormal _portalcamera (Math|Vector|GetForwardVector (Variables|Default|GetForwardDirection))))))

(fn Checkviewportsize
  (bind _returnvalue (Viewport|GetViewportSize))
  (bind _returnvalue_2 (Viewport|GetViewportSize))
  (bind _portal_rt (Variables|Default|GetPortal_RT))
  (bind (_x _y) (Math|Vector2D|BreakVector2D _returnvalue))
  (bind (_x_2 _y_2) (Math|Vector2D|BreakVector2D _returnvalue_2))
  (if (not (and (== _x (Variables|/Script/Engine.TextureRenderTarget2D|GetSizeX _portal_rt)) (== _y (Variables|/Script/Engine.TextureRenderTarget2D|GetSizeY _portal_rt))))
    (Development|PrintString "Resizing")
    (Rendering|ResizeRenderTarget2D (Variables|Default|GetPortal_RT) (Math|Float|Truncate _x_2) (Math|Float|Truncate _y_2))))

(fn ShouldTeleport?
  (Utilities|IsValid (Utilities|Array|Get(acopy) (Collision|GetOverlappingActors (Variables|Default|GetPlayerDetection) "/Game/LostRocket/Character/BP_FirstPersonCharacter.BP_FirstPersonCharacter_C" :!class /Script/Engine.PrimitiveComponent))
    (:Is%20Valid
      (bind _return (CallFunction|IsPointCrossingPortal? (Transformation|GetWorldLocation (Variables|/Game/LostRocket/Character/BP_FirstPersonCharacter.BP_FirstPersonCharacter_C|GetFirstPersonCamera (.AsBP%20First%20Person%20Character (Utilities|Casting|CastToBP_FirstPersonCharacter (Game|GetPlayerCharacter 0))))) (Transformation|GetActorLocation) (Math|Vector|GetForwardVector (Variables|Default|GetForwardDirection))))
      (if _return
        (Audio|Components|Audio|Play (Variables|Default|GetAudio) 0.0)
        (CallFunction|TeleportCharacter)))))

(fn IsPointCrossingPortal?
  (params (Point :type Vector) (PortalLocation :type Vector) (PortalNormal :type Vector))
  (LocalVariables|SetIsInFront (>= (Math|Vector|DotProduct PortalNormal (- Point PortalLocation)) 0.0))
  (bind _output_get (LocalVariables|SetPortalPlan (Class|KismetMathLibrary|MakePlanefromPointandNormal PortalLocation PortalNormal)))
  (bind _output_get_2 (LocalVariables|SetIs_Intersect (.ReturnValue (Class|KismetMathLibrary|LinePlaneIntersection (Variables|Default|GetLastPos) Point _output_get))))
  (Development|PrintString (Utilities|String|ToString(Boolean) _output_get_2) true true "(R=1.000000,G=0.096860,B=0.000000,A=1.000000)")
  (LocalVariables|SetIsCrossing (Math|Boolean|ANDBoolean (LocalVariables|GetIs_Intersect) (not (LocalVariables|GetIsInFront)) (Variables|Default|GetLastInFront)))
  (Variables|Default|SetLastInFront (LocalVariables|GetIsInFront))
  (Variables|Default|SetLastPos Point)
  (return (LocalVariables|GetIsCrossing)))

(fn TeleportCharacter
  (bind _returnvalue (Game|GetPlayerCharacter 0))
  (bind _returnvalue_2 (Transformation|GetActorTransform))
  (bind _returnvalue_3 (Transformation|GetActorTransform))
  (bind _returnvalue_4 (Game|GetPlayerController 0))
  (bind _returnvalue_5 (Transformation|GetActorTransform))
  (bind _returnvalue_6 (Game|GetPlayerCharacter 0))
  (bind _returnvalue_7 (Pawn|GetMovementComponent _returnvalue))
  (bind _returnvalue_8 (Transformation|GetActorRotation _returnvalue_4))
  (bind (_x _y _z) (Math|Vector|BreakVector (.scale _returnvalue_3)))
  (bind _returnvalue_9 (Transformation|GetActorRotation _returnvalue_6))
  (bind (_x_2 _y_2 _z_2) (Math|Rotator|GetAxes _returnvalue_8))
  (bind (_x_3 _y_3 _z_3) (Math|Rotator|GetAxes _returnvalue_9))
  (Transformation|SetActorTransform (Game|GetPlayerCharacter 0) (Math|Transform|MakeTransform (Math|Transform|TransformLocation (Transformation|GetActorTransform (Variables|Default|GetLinked%20portal)) (Math|Transform|InverseTransformLocation (Math|Transform|MakeTransform (.location _returnvalue_3) (.rotation _returnvalue_3) (Math|Vector|MakeVector (* _x -1.0) (* _y -1.0) _z)) (Transformation|GetActorLocation (Game|GetPlayerCharacter 0)))) (Math|Rotator|MakeRotationfromAxes (Math|Transform|TransformDirection (Transformation|GetActorTransform (Variables|Default|GetLinked%20portal)) (Math|Vector|MirrorVectorbyNormal (Math|Vector|MirrorVectorbyNormal (Math|Transform|InverseTransformDirection _returnvalue_5 _x_3) "1.000000,0.000000,0.000000") "0.000000,1.000000,0.000000")) (Math|Transform|TransformDirection (Transformation|GetActorTransform (Variables|Default|GetLinked%20portal)) (Math|Vector|MirrorVectorbyNormal (Math|Vector|MirrorVectorbyNormal (Math|Transform|InverseTransformDirection _returnvalue_5 _y_3) "1.000000,0.000000,0.000000") "0.000000,1.000000,0.000000")) (Math|Transform|TransformDirection (Transformation|GetActorTransform (Variables|Default|GetLinked%20portal)) (Math|Vector|MirrorVectorbyNormal (Math|Vector|MirrorVectorbyNormal (Math|Transform|InverseTransformDirection _returnvalue_5 _z_3) "1.000000,0.000000,0.000000") "0.000000,1.000000,0.000000"))) "1.000000,1.000000,1.000000"))
  (Pawn|SetControlRotation (Game|GetPlayerController 0) (Math|Rotator|MakeRotationfromAxes (Math|Transform|TransformDirection (Transformation|GetActorTransform (Variables|Default|GetLinked%20portal)) (Math|Vector|MirrorVectorbyNormal (Math|Vector|MirrorVectorbyNormal (Math|Transform|InverseTransformDirection _returnvalue_2 _x_2) "1.000000,0.000000,0.000000") "0.000000,1.000000,0.000000")) (Math|Transform|TransformDirection (Transformation|GetActorTransform (Variables|Default|GetLinked%20portal)) (Math|Vector|MirrorVectorbyNormal (Math|Vector|MirrorVectorbyNormal (Math|Transform|InverseTransformDirection _returnvalue_2 _y_2) "1.000000,0.000000,0.000000") "0.000000,1.000000,0.000000")) (Math|Transform|TransformDirection (Transformation|GetActorTransform (Variables|Default|GetLinked%20portal)) (Math|Vector|MirrorVectorbyNormal (Math|Vector|MirrorVectorbyNormal (Math|Transform|InverseTransformDirection _returnvalue_2 _z_2) "1.000000,0.000000,0.000000") "0.000000,1.000000,0.000000"))))
  (bind _returnvalue_10 (CallFunction|UpdateVelocity (Variables|/Script/Engine.MovementComponent|GetVelocity _returnvalue_7)))
  (Variables|/Script/Engine.MovementComponent|SetVelocity _returnvalue_7 _returnvalue_10)
  ;[1 1 1] if this is the portal at the end of the level, use the function tp end level to finish the level
  (if (Variables|Default|GetEndPortal)
    (bind _outactors (Actor|GetAllActorsOfClasswithTag "/Game/LostRocket/DynamicObject/ActorLevelPlatformer/BP_TimingSystem.BP_TimingSystem_C" "Tag"))
    (bind _asbp_first_person_character (Utilities|Casting|CastToBP_FirstPersonCharacter (Game|GetPlayerCharacter 0)))
    (Default|TpEndLevel _asbp_first_person_character (Variables|/Game/LostRocket/DynamicObject/ActorLevelPlatformer/BP_TimingSystem.BP_TimingSystem_C|GetTotalFuel (Utilities|Array|Get(acopy) _outactors)))))

(fn UpdateVelocity
  (params (Velocity :type Vector))
  (return (* (Math|Transform|TransformDirection (Transformation|GetActorTransform (Variables|Default|GetLinked%20portal)) (Math|Vector|MirrorVectorbyNormal (Math|Vector|MirrorVectorbyNormal (Math|Transform|InverseTransformDirection (Transformation|GetActorTransform) (Math|Vector|Normalize Velocity)) "1.000000,0.000000,0.000000") "0.000000,1.000000,0.000000")) (Math|Vector|VectorLength Velocity))))