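; Timed-challenge actor that sends the player back to a stored pre-portal location when its countdown runs out.
; Player overlap while elapsed time is zero starts a looping one-second timer and shows the countdown on the player's HUD.
; Each tick updates the remaining time; at the limit it clears the timer, moves the player, plays a teleport sound and passes zero to the HUD.
; Elapsed time is never reset in this graph.
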(event Custom|TimerEvent
  ;[1 1 1] increment the timer
  (Variables|Default|SetTimeActual (+ (Variables|Default|GetTimeActual) 1.0))
  (bind _output_get (Variables|Default|SetTimeLeft (- (Variables|Default|GetTimeMax) (Variables|Default|GetTimeActual))))
  (Development|PrintString (Utilities|String|ToString(Float) _output_get))
  (Default|UpdateTime (Variables|/Game/LostRocket/Character/BP_FirstPersonCharacter.BP_FirstPersonCharacter_C|GetWB_Player_Hud (Variables|Default|GetBP%20First%20Person%20Character)) (Variables|Default|GetTimeLeft))
  ;[1 1 1] if time is out stop the clock and do the rest
  (if (>= (Variables|Default|GetTimeActual) (Variables|Default|GetTimeMax))
    (Utilities|Time|ClearandInvalidateTimerbyHandle (Variables|Default|GetTimerHandler))
    (Transformation|SetActorLocation (Variables|Default|GetBP%20First%20Person%20Character) (Variables|Default|GetLocationBeforePortal) false false)
    (Audio|PlaySound2D "/Game/LostRocket/DynamicObject/Portal/S_TP_out.S_TP_out" 1.0 1.0 0.0 0 0)
    (Default|SetVisibleTime (Variables|/Game/LostRocket/Character/BP_FirstPersonCharacter.BP_FirstPersonCharacter_C|GetWB_Player_Hud (Variables|Default|GetBP%20First%20Person%20Character)) 0.0)))

(event Collision|EventActorBeginOverlap
  (params (OtherActor :type Actor%20Object%20Reference))
  ;[1 1 1] on touch if there is no timer, start a timer
  (bind _asbp_first_person_character (Utilities|Casting|CastToBP_FirstPersonCharacter OtherActor))
  (Variables|Default|SetBP%20First%20Person%20Character _asbp_first_person_character)
  (if (== (Variables|Default|GetTimeActual) 0.0)
    (bind _returnvalue (Utilities|Time|SetTimerbyEvent (delegate Custom|TimerEvent) 1.0 true))
    (Variables|Default|SetTimerHandler _returnvalue)
    (Default|SetVisibleTime (Variables|/Game/LostRocket/Character/BP_FirstPersonCharacter.BP_FirstPersonCharacter_C|GetWB_Player_Hud (Variables|Default|GetBP%20First%20Person%20Character)) (Variables|Default|GetTimeMax))))

(fn ConstructionScript)