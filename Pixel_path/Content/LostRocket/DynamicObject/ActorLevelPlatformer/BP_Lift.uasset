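; BP_Lift is a platformer lift that moves while the first-person character is overlapping it and returns after they leave.
; Overlap begin plays a timeline and overlap end reverses it, each after a short delay.
; The timeline's Lift track scales the offset from the actor's BeginPlay location to EndLocation, which sets the platform mesh's relative location without sweeping.
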(event EventBeginPlay
  (Variables|Default|SetBeginLocation (Transformation|GetActorLocation)))

(event Collision|EventActorBeginOverlap
  (params (OtherActor :type Actor%20Object%20Reference))
  (Utilities|Casting|CastToBP_FirstPersonCharacter OtherActor)
  (Utilities|FlowControl|Delay 0.2)
  (bind _lift (Timeline|Timeline Play)
    (:Update
      (Transformation|SetRelativeLocation (Variables|Default|GetSM_RoofConnector_3_Merged) (* _lift (- (Variables|Default|GetEndLocation) (Variables|Default|GetBeginLocation))) false false))))

(event Collision|EventActorEndOverlap
  (params (OtherActor :type Actor%20Object%20Reference))
  (Utilities|Casting|CastToBP_FirstPersonCharacter OtherActor)
  (Utilities|FlowControl|Delay 0.2)
  (bind _lift (Timeline|Timeline Reverse)
    (:Update
      (Transformation|SetRelativeLocation (Variables|Default|GetSM_RoofConnector_3_Merged) (* _lift (- (Variables|Default|GetEndLocation) (Variables|Default|GetBeginLocation))) false false))))

(fn ConstructionScript)