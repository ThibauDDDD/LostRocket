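; Spline-driven wall actor for the platformer level that tiles a mesh along a designer-placed spline.
; The construction script adds one spline mesh per mesh X-length step, with tangents clamped to that length.
; Each segment also gets a box collision at its start point plus a fixed offset, without spline rotation.
; Overlap with the first-person character only prints its name; no teleport logic exists despite the "Tp" name.
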(event EventBeginPlay)

(event Collision|EventActorBeginOverlap
  (params (OtherActor :type Actor%20Object%20Reference))
  (Utilities|Casting|CastToBP_FirstPersonCharacter OtherActor)
  (Development|PrintString (Utilities|GetDisplayName OtherActor)))

(event EventTick
  (params (DeltaSeconds :type Float%20%28single-precision%29)))

(fn ConstructionScript
  (bind _mesh (Variables|Default|GetMesh))
  (bind _spline (Variables|Default|GetSpline))
  (bind _spline_2 (Variables|Default|GetSpline))
  (bind _returnvalue (StaticMesh|GetBoundingBox _mesh))
  ;[1 1 1] set la mesh là où il faut (me demandez pas d'explications)
  (bind _output_get (Variables|Default|SetLength (.x (+ (Math|Vector|VectorGetAbs (.min _returnvalue)) (Math|Vector|VectorGetAbs (.max _returnvalue))))))
  (for _index (range 0 (Math|Float|Truncate (/ (Spline|GetSplineLength (Variables|Default|GetSpline)) _output_get)))
    (bind _returnvalue_2 (AddComponent|AddSplineMeshComponent false))
    (SplineMesh|SetForwardAxis _returnvalue_2 "X" true)
    (SplineMesh|SetStartandEnd _returnvalue_2 (Spline|GetLocationatDistanceAlongSpline _spline (* _index (Variables|Default|GetLength)) "Local") (Math|Vector|ClampVectorSize (Spline|GetTangentatDistanceAlongSpline _spline (* _index (Variables|Default|GetLength)) "Local") 0.0 (Variables|Default|GetLength)) (Spline|GetLocationatDistanceAlongSpline _spline_2 (* (+ _index 1) (Variables|Default|GetLength)) "Local") (Math|Vector|ClampVectorSize (Spline|GetTangentatDistanceAlongSpline _spline_2 (* (+ _index 1) (Variables|Default|GetLength)) "Local") 0.0 (Variables|Default|GetLength)) true :!class /Script/Engine.SplineMeshComponent)
    ;[1 1 1] add a collision to the wall
    (bind _returnvalue_3 (AddComponent|AddBoxComponent false))
    (bind _output_get_2 (Variables|Default|SetBoxCollision _returnvalue_3))
    (Transformation|SetRelativeLocation _returnvalue_3 (+ (Spline|GetLocationatDistanceAlongSpline _spline (* _index (Variables|Default|GetLength)) "Local") "0.000000,250.000000,40.000000") false false)))