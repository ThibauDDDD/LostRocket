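; BP_Ressource is a harvestable resource object that pays out to the player each time its mesh is hit.
; Each hit adds its amount to the first-person character's ARessource map under its resource type, whatever caused the hit.
; The hit also removes fixed health and spawns an explosion effect, then destroys the actor once health is depleted.
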(event OnComponentHit(Mesh)
  (params (HitComponent :type Primitive%20Component%20Object%20Reference) (OtherActor :type Actor%20Object%20Reference) (OtherComp :type Primitive%20Component%20Object%20Reference) (NormalImpulse :type Vector :default "0, 0, 0") (Hit :type Hit%20Result%20Structure%20%28by%20ref%29))
  (bind _asbp_first_person_character (Utilities|Casting|CastToBP_FirstPersonCharacter (Game|GetPlayerCharacter 0)))
  (Utilities|AddRsstoPlayer _asbp_first_person_character)
  (Utilities|RemoveHealth)
  (Effects|SpawnEmitteratLocation "/Game/StarterContent/Particles/P_Explosion.P_Explosion" (Transformation|GetActorLocation))
  (Utilities|DestroyActor))

(fn ConstructionScript)