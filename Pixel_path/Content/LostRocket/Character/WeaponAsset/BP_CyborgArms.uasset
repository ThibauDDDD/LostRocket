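; Cyborg arms weapon Blueprint for LostRocket, extending a parent weapon class by overriding its events.
; Shoot and reload feedback forward to server calls on the attach-parent actor.
; Draw spawns an actor snapped to a socket on that parent's mesh, and changing weapon destroys it when not drawing.
; Hit feedback calls a reticule event that is an empty TODO stub, with the HUD hit animation logic left disconnected.
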(event Custom|reticule)

(event EventBeginPlay
  (|CallParentFunction) ; This node is disabled and will not be called.\nDrag off pins to build functionality.
)

(event Collision|EventActorBeginOverlap
  (params (OtherActor :type Actor%20Object%20Reference)))

(event EventTick
  (params (DeltaSeconds :type Float%20%28single-precision%29)))

(event EventDraw
  (bind _returnvalue (Actor|GetAttachParentActor))
  (bind _asbp_my_character (Utilities|Casting|CastTo _returnvalue))
  (|CallParentFunction)
  (bind _returnvalue_2 (Game|SpawnActorfromClass (Variables|Default|GetActor) (Transformation|GetActorTransform _asbp_my_character) "AlwaysSpawn" "MultiplyWithRoot" 0 0))
  (bind _output_get (Variables|Default|SetActorRef _returnvalue_2))
  (Utilities|IsValid _output_get
    (:Is%20Valid
      (Transformation|AttachComponentToComponent _output_get (Variables|/Script/Engine.Character|GetMesh _asbp_my_character) (Variables|Default|GetSocketName) "SnapToTarget" "SnapToTarget" "SnapToTarget" true)
      (Actor|SetOwner _output_get _asbp_my_character))))

(event EventDamageableHitFeedbackAll
  (params (Location :type Vector :default "0, 0, 0") (Damages :type Float%20%28double-precision%29))
  (|CallParentFunction Location Damages)
  (CallFunction|Reticule))

(event EventReloadingFeedback
  (|CallParentFunction)
  (CallFunction|ReloadServer (.AsBP%20My%20Character (Utilities|Casting|CastTo (Actor|GetAttachParentActor)))))

(event EventOnChangingWeapon
  (bind _actorref (Variables|Default|GetActorRef))
  (|CallParentFunction)
  (if (not (Variables|Default|GetIsDrawing?))
    (Utilities|IsValid _actorref
      (:Is%20Valid
        (Actor|DestroyActor _actorref)))))

(event EventShoot
  (|CallParentFunction)
  (CallFunction|ShootServer (.AsBP%20My%20Character (Utilities|Casting|CastTo (Actor|GetAttachParentActor)))))

(fn ConstructionScript
  (|CallParentFunction))